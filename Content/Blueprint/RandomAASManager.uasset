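; RandomAASManager builds a randomized AAS capture lattice on the server at BeginPlay, running from Team One main to Team Two main.
; It groups capzones by their distinct CapzonesLayer values and picks a random zone from each layer.
; Each pick is chained to the previous node as a link in LatticeActor's Lattice, ending at Team Two main.
; Unpicked capzones are collected and destroyed once the chain is complete.
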(event `self.ReceiveBeginPlay`
  (bind _capzones__layer (`self.Capzones /Layer`))
  (bind _tempcaplist (`self.TempCapList`))
  (bind _length (`self.Length`))
  (bind _output (`|GetArrayItem` _tempcaplist (`KismetMathLibrary.RandomInteger` (`KismetArrayLibrary.Array_Length` _tempcaplist))))
  (`/Engine/EditorBlueprintResources/ActorMacros.Switch Has Authority`
    (:`Authority`
      (bind _values (`BlueprintMapLibrary.Map_Values` (`self.Capzones /Layer`)))
      (for _array_element _values
        (`KismetArrayLibrary.Array_AddUnique` _length _array_element))
      (set `self.FirstLink` (`self.Team One Main`))
      (for _array_element_2 _length
        (bind _keys (`BlueprintMapLibrary.Map_Keys` _capzones__layer))
        (for _array_element_3 _keys
          (bind (_value _returnvalue) (`BlueprintMapLibrary.Map_Find` _capzones__layer _array_element_3))
          (if _returnvalue
            (if (== _array_element_2 _value)
              (`KismetArrayLibrary.Array_Add` (`self.TempCapList`) _array_element_3))
            (else
              (`KismetSystemLibrary.PrintString` "Badkey"))))
        (`/Engine/EditorBlueprintResources/StandardMacros.IsValid` _output
          (:`Is Valid`
            (set `self.SecondLink` _output)
            (`KismetArrayLibrary.Array_Add` (`SQAASLattice.Lattice` (`self.Lattice Actor`)) (make `SQAASLatticeLink` (`self.FirstLink`) (`self.SecondLink`)))
            (`/Engine/EditorBlueprintResources/ActorMacros.Switch Has Authority`
              (:`Authority`
                (bind _output_get (set `self.FirstLink` (`self.SecondLink`))))))
          (:`Is Not Valid`
            (`KismetSystemLibrary.PrintString` "NOVALID" true true (struct :`G` 0.66 :`B` 1.0 :`A` 1.0) 99999.0)))
        (for _array_element_4 (`self.TempCapList`)
          (if (!= _output_get _array_element_4)
            (`KismetArrayLibrary.Array_Add` (`self.AlreadyDone`) _array_element_4)))
        (`KismetArrayLibrary.Array_Clear` (`self.TempCapList`)))
      (set `self.SecondLink` (`self.Team Two Main`))
      (`KismetArrayLibrary.Array_Add` (`SQAASLattice.Lattice` (`self.Lattice Actor`)) (make `SQAASLatticeLink` (`self.FirstLink`) (`self.SecondLink`)))
      (for _array_element_5 (`self.AlreadyDone`)
        (`self.K2_DestroyActor` _array_element_5)))))

(fn `UserConstructionScript`)